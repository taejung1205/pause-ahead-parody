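; Game mode that runs a per-level countdown for the side-scroller character and respawns the player when time runs out.
; Tick uses a short Delay to step Timer down unless IsPaused is set, then destroys the character once it drops below zero.
; Respawn waits briefly, resets Timer from LevelTimerList by CurrentLevel, spawns the same character class at a player start and possesses it.
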(event Custom|Respawn
  (params (Player :type Character%20Object%20Reference))
  ;[1 1 1] Respawn
  (Utilities|FlowControl|Delay 1.0)
  (Variables|Default|SetTimer (Utilities|Array|Get(acopy) (Variables|Default|GetLevelTimerList) (Variables|Default|GetCurrentLevel)))
  (bind _returnvalue (Game|SpawnActorfromClass (Utilities|GetClass Player) (Transformation|GetActorTransform (Class|GameModeBase|FindPlayerStart)) "Undefined" 0 0))
  (Pawn|Possess (Game|GetPlayerController 0) _returnvalue))

(event EventBeginPlay)

(event EventTick
  (params (DeltaSeconds :type Float%20%28single-precision%29))
  ;[1 1 1] Timer
  (Utilities|FlowControl|Delay 0.1)
  (if (not (Variables|Default|GetIsPaused))
    (if (< (Variables|Default|GetTimer) 0.0)
      ;[1 1 1] Time over
      (bind _asside_scroller_character (Utilities|Casting|CastToSideScrollerCharacter (Game|GetPlayerCharacter 0)))
      (Actor|DestroyActor _asside_scroller_character)
      (CallFunction|Respawn _asside_scroller_character)
      (else
        (Variables|Default|SetTimer (- (Variables|Default|GetTimer) 0.1))))))

(fn ConstructionScript)